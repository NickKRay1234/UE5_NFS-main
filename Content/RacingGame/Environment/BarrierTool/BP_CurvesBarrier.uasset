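; BP_CurvesBarrier is a construction-time tool that places copies of a selectable mesh along a spline, for building barriers in the racing game.
; Its construction script assigns MeshToSpawn to an instanced static mesh component, then adds one instance at each spline point in local space.
; Instances use only point locations, with zero rotation and unit scale, so they do not follow the curve's direction or fill gaps between points.
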(event EventBeginPlay)

(event Collision|EventActorBeginOverlap
  (params (OtherActor :type Actor%20Object%20Reference)))

(event EventTick
  (params (DeltaSeconds :type Float%20%28single-precision%29)))

(fn ConstructionScript
  (Components|StaticMesh|SetStaticMesh (Variables|Default|GetInstancedStaticMesh) (Variables|Default|GetMeshToSpawn))
  (for _index (range 0 (- (Spline|GetNumberOfSplinePoints (Variables|Default|GetSpline)) 1))
    (Components|InstancedStaticMesh|AddInstance (Variables|Default|GetInstancedStaticMesh) (Math|Transform|MakeTransform (.Location (Spline|GetLocationandTangentatSplinePoint (Variables|Default|GetSpline) _index "Local"))) false)))